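; BP_SpookyShadow01 is a one-shot scare that plays a spotlit shadow trick when the SpyGame character overlaps it.
; The overlap disables the Sphere's collision, then random delays time two one-second spotlight blackouts.
; The first blackout rotates the skeletal mesh 90 degrees in darkness.
; The second turns off its hidden-shadow casting as the light returns, removing any shadow cast while hidden.
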(event EventBeginPlay)

(event Collision|EventActorBeginOverlap
  (params (OtherActor :type Actor%20Object%20Reference))
  (Utilities|Casting|CastToBP_SpyGame_Character OtherActor)
  (Collision|SetCollisionEnabled (Variables|Default|GetSphere) "NoCollision")
  (Utilities|FlowControl|Delay (Math|Random|RandomFloatinRange 5.0 8.0))
  (Rendering|Components|Light|SetIntensity (Variables|Default|GetSpotLight) 0.0)
  (Transformation|SetRelativeRotation (Variables|Default|GetSkeletalMesh) "0,-90.000000, 0" false false)
  (Utilities|FlowControl|Delay 1.0)
  (Rendering|Components|Light|SetIntensity (Variables|Default|GetSpotLight) 1e+05)
  (Utilities|FlowControl|Delay (Math|Random|RandomFloatinRange 5.0 15.0))
  (Rendering|Components|Light|SetIntensity (Variables|Default|GetSpotLight) 0.0)
  (Utilities|FlowControl|Delay 1.0)
  (Class|PrimitiveComponent|SetCastHiddenShadow (Variables|Default|GetSkeletalMesh) false)
  (Rendering|Components|Light|SetIntensity (Variables|Default|GetSpotLight) 1e+05))

(event EventTick
  (params (DeltaSeconds :type Float%20%28single-precision%29)))

(fn ConstructionScript)