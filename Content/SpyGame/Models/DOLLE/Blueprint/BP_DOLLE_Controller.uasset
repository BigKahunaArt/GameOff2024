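; AI controller for the DOLLE enemy that patrols, hunts the spy player and can be summoned to a location.
; A Tick-driven state machine switches between Idle, Patrolling, Chasing and Summon using timers, driving AIMoveTo, speed, eye color and barks.
; Chasing starts on a forward sphere-trace sighting of an unhidden player, on fast player movement regardless of sight, or when a summon move ends.
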(event Custom|SummonDolle
  (params (Location :type Vector))
  (CallFunction|SetState "NewEnumerator6")
  (AI|AIMoveTo (Variables|Default|GetDollePawn) Location 0 5.0 false
    (:OnSuccess
      _)
    (:OnFail
      _))
  (CallFunction|SetState "NewEnumerator2"))

(event EventBeginPlay
  (bind _asbp_dolle_character (Utilities|Casting|CastToBP_DOLLE_Character (Pawn|GetControlledPawn)))
  (Variables|Default|SetDollePawn _asbp_dolle_character)
  (CallFunction|SetState "NewEnumerator0")
  (bind _asbp_spy_game_character (Utilities|Casting|CastToBP_SpyGame_Character (Pawn|GetControlledPawn (Game|GetPlayerController 0))))
  (Variables|Default|SetPlayer _asbp_spy_game_character))

(event EventTick
  (params (DeltaSeconds :type Float%20%28single-precision%29))
  (bind _dollepawn (Variables|Default|GetDollePawn))
  (bind _player (Variables|Default|GetPlayer))
  (bind _dollepawn_2 (Variables|Default|GetDollePawn))
  (bind _dollepawn_3 (Variables|Default|GetDollePawn))
  (if (Variables|/Game/SpyGame/Models/DOLLE/Blueprint/BP_DOLLE_Character.BP_DOLLE_Character_C|GetIsReady (Variables|Default|GetDollePawn))
    (if (> (Math|Vector|VectorLength (Transformation|GetVelocity (Variables|Default|GetPlayer))) 2.5e+02)
      (CallFunction|SetState "NewEnumerator2"))
    (bind _output_get (Variables|Default|Set_Counter (+ DeltaSeconds (Variables|Default|Get_Counter))))
    (if (> _output_get 3e+01)
      (CallFunction|SetState "NewEnumerator0"))
    (switch Utilities|FlowControl|Switch|SwitchonE_DolleState (Variables|Default|GetState)
      (:NewEnumerator0
        (bind _canseeplayer (CallFunction|CanSeePlayer))
        (if _canseeplayer
          (CallFunction|SetState "NewEnumerator2")
          (else
            (Default|SetEyeColor (Variables|Default|GetDollePawn) 1e+01 "(R=0.000000,G=0.853474,B=1.000000,A=1.000000)")
            (if (>= (Variables|Default|Get_Counter) 5.0)
              (CallFunction|SetState "NewEnumerator1")
              (else
                (AI|Navigation|StopMovement))))))
      (:NewEnumerator1
        (bind _canseeplayer_2 (CallFunction|CanSeePlayer))
        ;[1 1 1] Patrolling
        (if _canseeplayer_2
          (CallFunction|SetState "NewEnumerator2")
          (elif (<= (Math|Vector|VectorLength (Variables|/Script/Engine.MovementComponent|GetVelocity (Variables|/Script/Engine.Character|GetCharacterMovement _dollepawn))) 5.0)
            (bind _output_get_2 (Variables|Default|Set_PatrolIdleTime (+ DeltaSeconds (Variables|Default|Get_PatrolIdleTime))))
            (if (>= _output_get_2 5.0)
              (Utilities|FlowControl|DoOnce false :!label _label
                (:Completed
                  (bind _location (Default|GetRandomPatrolPoint _dollepawn))
                  (Default|SetEyeColor (Variables|Default|GetDollePawn) 1e+01 "(R=1.000000,G=0.509704,B=0.000000,A=1.000000)")
                  (AI|AIMoveTo _dollepawn _location 0 5.0 false
                    (:OnSuccess
                      _)
                    (:OnFail
                      _))
                  (Variables|Default|Set_Counter 0.0)
                  (Variables|Default|Set_PatrolIdleTime 0.0)
                  (goto _label Reset)))))))
      (:NewEnumerator2
        ;[1 1 1] Chasing
        (bind _canseeplayer_3 (CallFunction|CanSeePlayer))
        (if _canseeplayer_3
          (Default|SetFastMovementSpeed (Variables|Default|GetDollePawn))
          (Default|BarkSpotted _dollepawn_3)
          (Default|SetEyeColor _dollepawn_3 1e+02 "(R=1.000000,G=0.000000,B=0.000000,A=1.000000)")
          (AI|AIMoveTo (Variables|Default|GetDollePawn) (Transformation|GetActorLocation _player) _player 5.0 false)
          (else
            (bind _output_get_3 (Variables|Default|Set_LostPlayerTime (+ DeltaSeconds (Variables|Default|Get_LostPlayerTime))))
            (if (>= _output_get_3 (Math|Random|RandomFloatinRange 1e+01 15.0))
              (CallFunction|SetState "NewEnumerator0")
              (else
                (AI|AIMoveTo _dollepawn_2 (+ (Transformation|GetActorLocation (Variables|Default|GetPlayer)) (* (Math|Vector|GetRightVector (Variables|/Script/Engine.Character|GetMesh _dollepawn_2)) 1.5e+02)) 0 5.0 false))))))
      (:NewEnumerator6
        (bind _canseeplayer_4 (CallFunction|CanSeePlayer))
        (if _canseeplayer_4
          (CallFunction|SetState "NewEnumerator2"))))))

(fn ConstructionScript)

(fn GetPlayerDirection
  (bind _returnvalue (Game|GetPlayerCharacter 0))
  (bind _dollepawn (Variables|Default|GetDollePawn))
  (bind _returnvalue_2 (Transformation|GetActorLocation _dollepawn))
  (bind _returnvalue_3 (Transformation|GetActorLocation _returnvalue))
  (bind _returnvalue_4 (- _returnvalue_3 _returnvalue_2))
  (bind (_x _y _z) (Math|Vector|BreakVector _returnvalue_4))
  (return (Math|Vector|MakeVector _x _y _z)))

(fn SetState
  (params (New%20State :type E_DolleState%20Enum :default "NewEnumerator0"))
  (if (Utilities|Enum|Equal(Enum) New%20State (Variables|Default|GetState))
    (return)
    (else
      (bind _output_get (Variables|Default|SetState New%20State))
      (Variables|Default|Set_Counter 0.0)
      (Variables|Default|Set_LostPlayerTime 0.0)
      (Variables|Default|Set_PatrolIdleTime 0.0)
      (Development|PrintString (Utilities|String|EnumtoString _output_get))
      (Default|ResetMovementSpeed (Variables|Default|GetDollePawn))
      (return))))

(fn CanSeePlayer
  (bind _dollepawn (Variables|Default|GetDollePawn))
  (bind _returnvalue (Transformation|GetActorLocation _dollepawn))
  (bind (_outhit _returnvalue_2) (Collision|SphereTraceByChannel _returnvalue (+ _returnvalue (* (Math|Vector|GetRightVector (Variables|/Script/Engine.Character|GetMesh _dollepawn)) (Variables|Default|GetSightRange))) 1e+02 "TraceTypeQuery3" true 0 "ForOneFrame"))
  (if _returnvalue_2
    (bind _asbp_spy_game_character (Utilities|Casting|CastToBP_SpyGame_Character (.HitActor (Collision|BreakHitResult _outhit)))
      (:then
        (bind _hidden (Default|PlayerIsHidden _asbp_spy_game_character))
        (if _hidden
          (return false)
          (else
            (return true))))
      (:CastFailed
        (return false)))
    (else
      (return false))))