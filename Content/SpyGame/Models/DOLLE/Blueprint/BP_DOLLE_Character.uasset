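; BP_DOLLE_Character is the DOLLE enemy character, which ends the game and destroys itself when it overlaps an unhidden player.
; Once ready, it barks on a random-interval looping timer, toggles movement audio by velocity, and forwards summon requests to BP_DOLLE_Controller, retrying until ready.
; It also exposes helpers for random patrol points, dynamic-material eye color, walk speed changes and a spotted sound.
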(event Custom|Bark
  (if (Variables|Default|GetIsReady)
    (Audio|PlaySoundatLocation "/Game/SpyGame/SFX/DOLLE_Barks.DOLLE_Barks" (Transformation|GetActorLocation) "0, 0, 0" 1.5 1.0 0.0 "/Game/SpyGame/SFX/SoundAttenuation.SoundAttenuation" "/Game/SpyGame/SFX/BarkConcurrency.BarkConcurrency" 0)))

(event Custom|Bark_Spotted
  (Audio|PlaySoundatLocation "/Game/SpyGame/SFX/DOLLE_Spotted.DOLLE_Spotted" (Transformation|GetActorLocation) "0, 0, 0" 2.5 1.0 0.0 "/Game/SpyGame/SFX/SoundAttenuation.SoundAttenuation" "/Game/SpyGame/SFX/BarkConcurrency.BarkConcurrency" 0))

(event Custom|Event_Ready
  (Variables|Default|SetIsReady true))

(event EventBeginPlay
  (bind _returnvalue (Rendering|Material|CreateDynamicMaterialInstance (Variables|Character|GetMesh) 2 0 "None" :!class /Script/Engine.PrimitiveComponent))
  (Variables|Default|Set_EyeMaterial _returnvalue)
  (Utilities|Time|SetTimerbyEvent (delegate Custom|Bark) (Math|Random|RandomFloatinRange 8.0 2e+01) true)
  (Class|AudioComponent|SetPaused (Variables|Default|GetDOLLE_Movement) (not (Variables|Default|GetIsReady))))

(event Collision|EventActorBeginOverlap
  (params (OtherActor :type Actor%20Object%20Reference))
  (bind _asbp_spy_game_character (Utilities|Casting|CastToBP_SpyGame_Character OtherActor))
  (Variables|Default|SetPlayer _asbp_spy_game_character))

(event EventTick
  (params (DeltaSeconds :type Float%20%28single-precision%29))
  (bind _dolle_movement (Variables|Default|GetDOLLE_Movement))
  (if (Variables|Default|GetIsReady)
    (Utilities|FlowControl|Sequence
      (:then_0
        (if (> (Math|Vector|VectorLength (Variables|/Script/Engine.MovementComponent|GetVelocity (Variables|Character|GetCharacterMovement))) 5.0)
          (Class|AudioComponent|SetPaused _dolle_movement false)
          (else
            (Class|AudioComponent|SetPaused _dolle_movement true))))
      (:then_1
        (bind _player (Variables|Default|GetPlayer)
          (:then
            (bind _hidden (Default|PlayerIsHidden _player))
            (if (not _hidden)
              (Default|GameOver (Variables|Default|GetPlayer) "NewEnumerator4")
              (Actor|DestroyActor)))
          (:else))))))

(event Collision|EventActorEndOverlap
  (params (OtherActor :type Actor%20Object%20Reference))
  (Utilities|Casting|CastToBP_SpyGame_Character OtherActor)
  (Variables|Default|SetPlayer 0))

(event EventActivate
  (Variables|Default|SetIsLaying false))

(event EventSummonto
  (params (Location :type Vector :default "0, 0, 0"))
  (if (Variables|Default|GetIsReady) :!label _label
    (bind _asbp_dolle_controller (Utilities|Casting|CastToBP_DOLLE_Controller (Pawn|GetController)))
    (Default|SummonDolle _asbp_dolle_controller Location)
    (else
      (Utilities|FlowControl|Delay 0.2)
      (goto _label))))

(fn ConstructionScript)

(fn GetRandomPatrolPoint
  (bind _patrolpoints (Variables|Default|GetPatrolPoints))
  (Development|PrintString "Getting random patrol point")
  (return (Transformation|GetActorLocation (Utilities|Array|Get(acopy) _patrolpoints (Math|Random|RandomInteger (Utilities|Array|Length _patrolpoints))))))

(fn SetEyeColor
  (params (Power :type Float%20%28single-precision%29) (Color :type Linear%20Color%20Structure))
  (bind __eyematerial (Variables|Default|Get_EyeMaterial))
  (Rendering|Material|SetScalarParameterValue __eyematerial "Power" Power :!class /Script/Engine.MaterialInstanceDynamic)
  (Rendering|Material|SetVectorParameterValue __eyematerial "Color" Color :!class /Script/Engine.MaterialInstanceDynamic)
  (return))

(fn ResetMovementSpeed
  (Variables|/Script/Engine.CharacterMovementComponent|SetMaxWalkSpeed (Variables|Character|GetCharacterMovement) 2.2e+02))

(fn SetFastMovementSpeed
  (Variables|/Script/Engine.CharacterMovementComponent|SetMaxWalkSpeed (Variables|Character|GetCharacterMovement) 2.8e+02))