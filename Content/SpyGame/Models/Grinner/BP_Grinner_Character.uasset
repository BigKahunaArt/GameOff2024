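; BP_Grinner_Character is the Grinner character Blueprint, which periodically plays a laugh sound at its location.
; BeginPlay records the starting position and starts a looping timer, with a random interval picked once, that fires the Bark event and its debug print.
; Tick is empty: disconnected leftover logic holds a vertical jiggle and an interpolated back-and-forth patrol around the start point, neither of which runs.
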(event Custom|Bark
  (Audio|PlaySoundatLocation "/Game/SpyGame/SFX/Grinner_Laugh_Rand.Grinner_Laugh_Rand" (Transformation|GetActorLocation) "0, 0, 0" 1.0 1.0 0.0 0 0 0)
  (Development|PrintString "Grinner bark"))

(event EventBeginPlay
  (bind _output_get (Variables|Default|SetTarget (Transformation|GetActorLocation)))
  (Variables|Default|SetStartingPosition _output_get)
  (Utilities|Time|SetTimerbyEvent (delegate Custom|Bark) (Math|Random|RandomFloatinRange 1e+01 2e+01) true))

(event Collision|EventActorBeginOverlap
  (params (OtherActor :type Actor%20Object%20Reference)))

(event EventTick
  (params (DeltaSeconds :type Float%20%28single-precision%29)))

(fn ConstructionScript)