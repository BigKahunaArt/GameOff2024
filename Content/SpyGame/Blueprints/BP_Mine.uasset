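; BP_Mine is a motion-sensitive mine that ends the game for a BP_SpyGame_Character caught in its blast.
; Overlap events track that character, and Tick triggers Explode when its speed exceeds BombThreshold, so slow movement is safe.
; Activate also detonates it directly.
; Explode fires once, sphere-traces pawns for GameOver, then plays sound and Niagara and hides mesh and danger ring, skipping these effects if the hit pawn fails the cast.
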(event Custom|Explode
  (bind _returnvalue (Transformation|GetActorLocation))
  (if (not (Variables|Default|GetIsDead))
    (Variables|Default|SetIsDead true)
    (bind (_outhit _returnvalue_2) (Collision|SphereTraceForObjects _returnvalue _returnvalue (Variables|Default|GetExplosionRadius) (Utilities|Array|MakeArray "ObjectTypeQuery3") true 0 "None"))
    (if _returnvalue_2
      (bind _asbp_spy_game_character (Utilities|Casting|CastToBP_SpyGame_Character (.HitActor (Collision|BreakHitResult _outhit))))
      (Default|GameOver _asbp_spy_game_character "NewEnumerator3"))
    (Audio|PlaySoundatLocation "/Game/SpyGame/SFX/Explosion_classic_1.Explosion_classic_1" (Transformation|GetActorLocation) "0, 0, 0" 1.0 1.0 0.0 0 0 0)
    (Rendering|SetVisibility (Variables|Default|Getprop-mine-01) false false)
    (Rendering|SetVisibility (Variables|Default|GetNS_DangerRing) false false)
    (Components|Activation|Activate (Variables|Default|GetNS_Explosion) true)))

(event EventBeginPlay)

(event Collision|EventActorBeginOverlap
  (params (OtherActor :type Actor%20Object%20Reference))
  (bind _asbp_spy_game_character (Utilities|Casting|CastToBP_SpyGame_Character OtherActor))
  (Variables|Default|SetPlayerCharacter _asbp_spy_game_character))

(event EventTick
  (params (DeltaSeconds :type Float%20%28single-precision%29))
  (Variables|Default|GetPlayerCharacter
    (:then
      (if (and (> (Math|Vector|VectorLength (Transformation|GetVelocity (Variables|Default|GetPlayerCharacter))) (Variables|Default|GetBombThreshold)) (not (Variables|Default|GetIsDead)))
        (CallFunction|Explode)))
    (:else)))

(event Collision|EventActorEndOverlap
  (params (OtherActor :type Actor%20Object%20Reference))
  (Utilities|Casting|CastToBP_SpyGame_Character OtherActor)
  (Variables|Default|SetPlayerCharacter 0))

(event EventActivate
  (CallFunction|Explode))

(fn ConstructionScript)