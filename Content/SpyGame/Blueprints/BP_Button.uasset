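; BP_Button is an interactable button station that temporarily toggles a linked Door when activated.
; BeginPlay creates a dynamic material on the station mesh as its indicator light and sets it red.
; ActivatewithNotify plays a sound, waits a short random delay, toggles the Door, turns the light green and tells the Notifier the interaction is complete.
; After CloseDelay it toggles the Door again and restores the red light.
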(event EventBeginPlay
  (|CallParentFunction)
  (bind _returnvalue (Rendering|Material|CreateDynamicMaterialInstance (Variables|Default|Getbutton-station) 2 0 "None" :!class /Script/Engine.PrimitiveComponent))
  (Variables|Default|SetLightMaterial _returnvalue)
  (Rendering|Material|SetVectorParameterValue _returnvalue "Color" "(R=1.000000,G=0.000000,B=0.000000,A=1.000000)" :!class /Script/Engine.MaterialInstanceDynamic))

(event Collision|EventActorBeginOverlap
  (params (OtherActor :type Actor%20Object%20Reference))
  (|CallParentFunction OtherActor) ; This node is disabled and will not be called.\nDrag off pins to build functionality.
)

(event EventTick
  (params (DeltaSeconds :type Float%20%28single-precision%29))
  (|CallParentFunction DeltaSeconds) ; This node is disabled and will not be called.\nDrag off pins to build functionality.
)

(event EventActivatewithNotify
  (params (Notifier :type I%20Notifier%20Interface))
  (bind _door (Variables|Default|GetDoor))
  (Audio|PlaySoundatLocation "/Game/SpyGame/SFX/button-202966_Cue.button-202966_Cue" (Transformation|GetActorLocation) "0, 0, 0" 1.0 1.0 0.0 0 0 0)
  (Utilities|FlowControl|Delay (Math|Random|RandomFloatinRange 0.1 0.5))
  (Default|Toggle _door)
  (CallFunction|SetLightColor "(R=0.046233,G=1.000000,B=0.000000,A=1.000000)")
  (Default|InteractionComplete Notifier)
  (Utilities|FlowControl|Delay (Variables|Default|GetCloseDelay))
  (Default|Toggle _door)
  (CallFunction|SetLightColor "(R=1.000000,G=0.000000,B=0.000000,A=1.000000)"))

(fn ConstructionScript
  (|CallParentFunction))

(fn SetLightColor
  (params (Color :type Linear%20Color%20Structure))
  (Rendering|Material|SetVectorParameterValue (Variables|Default|GetLightMaterial) "Color" Color :!class /Script/Engine.MaterialInstanceDynamic)
  (return))