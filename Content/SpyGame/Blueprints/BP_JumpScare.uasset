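; BP_JumpScare is an actor that plays a doll jump scare and triggers game over for the player's spy character.
; At BeginPlay it teleports far below the world origin and hides itself.
; Activate only sets a flag, which Tick polls and clears before revealing the actor and switching the player's view target to it.
; It then plays the scare sound and doll animation, and calls GameOver on the character after a short delay.
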(event EventTick
  (params (DeltaSeconds :type Float%20%28single-precision%29))
  (bind _returnvalue (Game|GetPlayerController 0))
  ;[1 1 1] It might be better to cache this inside the level blueprint?
  (if (Variables|Default|GetIsActive)
    (Variables|Default|SetIsActive false)
    (Rendering|SetVisibility (Variables|Default|GetDefaultSceneRoot) true true)
    (bind _asbp_spy_game_character (Utilities|Casting|CastToBP_SpyGame_Character (Pawn|GetControlledPawn _returnvalue)))
    (Game|Player|SetViewTargetwithBlend _returnvalue self 0.0 "VTBlend_Linear" 0.0 false)
    (Audio|PlaySound2D "/Game/SpyGame/SFX/jump-scares-2-159305_Cue.jump-scares-2-159305_Cue" 1.0 1.0 0.0 0 0)
    (Components|Animation|PlayAnimation (Variables|Default|GetDOLLE) "/Game/SpyGame/Models/DOLLE/anims/DOLLE_Jumpscare_01.DOLLE_Jumpscare_01" false)
    (Utilities|FlowControl|Delay 0.1)
    (Default|GameOver _asbp_spy_game_character "NewEnumerator4")))

(event EventBeginPlay
  (Transformation|SetActorLocation "0, 0,-5000.000000" false true)
  (Rendering|SetVisibility (Variables|Default|GetDefaultSceneRoot) false true))

(fn ConstructionScript)

(fn Activate
  (Variables|Default|SetIsActive true)
  (return))