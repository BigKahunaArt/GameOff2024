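; Factory wall Blueprint that builds a modular wall from instanced copies of a single static mesh.
; The construction script clamps the wall count to a small range, then uses nested loops to add instances in a grid along local X and Z at fixed spacing.
; The column loop is inclusive, so it places one more column than the count, while wall height sets the rows.
; The event graph has no active logic.
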(event EventBeginPlay)

(event Collision|EventActorBeginOverlap
  (params (OtherActor :type Actor%20Object%20Reference)))

(event EventTick
  (params (DeltaSeconds :type Float%20%28single-precision%29)))

(fn ConstructionScript
  (bind _output_get (Variables|Default|SetWallCount (Math|Integer|Clamp(Integer) (Variables|Default|GetWallCount) 0 5)))
  (for _index (range 0 _output_get)
    ;[1 1 1] Build Wall
    (for _index_2 (range 0 (- (Variables|Default|GetWallHeight) 1))
      (Components|InstancedStaticMesh|AddInstance (Variables|Default|GetInstancedStaticMesh) (Math|Transform|MakeTransform (Math|Vector|MakeVector (* _index 403.0) 0.0 (* _index_2 2e+02)) "0, 0, 0" "1,1,1")))))