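; BP_FactoryFloor is a construction-script actor that lays out a row of repeated factory floor pieces.
; The construction script clamps the floor count to a small range, then loops to add instances of the floor mesh to one instanced static mesh component.
; Each instance is offset along Y by the mesh length and given a shared scale.
; The event graph holds no active logic.
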(event EventBeginPlay)

(event Collision|EventActorBeginOverlap
  (params (OtherActor :type Actor%20Object%20Reference)))

(event EventTick
  (params (DeltaSeconds :type Float%20%28single-precision%29)))

(fn ConstructionScript
  (bind _instancedstaticmesh (Variables|Default|GetInstancedStaticMesh))
  (Variables|Default|SetFloorCount (Math|Integer|Clamp(Integer) (Variables|Default|GetFloorCount) 1 10))
  ;[1 1 1] Build Wall
  (for _index (range 0 (Variables|Default|GetFloorCount))
    (Components|StaticMesh|SetStaticMesh _instancedstaticmesh (Variables|Default|GetFloorMesh))
    (Components|InstancedStaticMesh|AddInstance _instancedstaticmesh (Math|Transform|MakeTransform (Math|Vector|MakeVector 0.0 (* _index (Variables|Default|GetMeshLength)) 0.0) "0, 0, 0" (Math|Conversions|ToVector(Float) (Variables|Default|GetScale))))))