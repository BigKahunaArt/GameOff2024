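; BP_FadeIn is a one-shot actor that fades the view in through a post-process material, then destroys itself.
; BeginPlay creates a dynamic instance of PP_FadeOut, adds it to the PostProcess component at full opacity, and starts the fade after a short delay.
; Tick lowers Opacity by FadeInSpeed until it reaches zero.
; Activate sets that speed and starts the fade immediately.
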(event EventBeginPlay
  (bind _output_get (Variables|Default|Set_Alpha 1.0))
  (bind _returnvalue (Rendering|Material|CreateDynamicMaterialInstance "/Game/SpyGame/Engine/PostProcessing/PP_FadeOut.PP_FadeOut" "None" "None" :!class /Script/Engine.KismetMaterialLibrary))
  (bind _output_get_2 (Variables|Default|SetPostProcessMaterial _returnvalue))
  (Rendering|Material|SetScalarParameterValue _output_get_2 "Opacity" _output_get :!class /Script/Engine.MaterialInstanceDynamic)
  (Rendering|AddorUpdateBlendable (Variables|Default|GetPostProcess) _output_get_2 1.0 :!class /Script/Engine.PostProcessComponent)
  (Utilities|FlowControl|Delay 0.2)
  (Variables|Default|SetIsActive true))

(event EventTick
  (params (DeltaSeconds :type Float%20%28single-precision%29))
  (if (Variables|Default|GetIsActive)
    (bind _output_get (Variables|Default|Set_Alpha (- (Variables|Default|Get_Alpha) (* DeltaSeconds (Variables|Default|Get_FadeInSpeed)))))
    (if (<= _output_get 0.0)
      (Variables|Default|SetIsActive false)
      (Variables|Default|Set_Alpha 0.0)
      (Rendering|Material|SetScalarParameterValue (Variables|Default|GetPostProcessMaterial) "Opacity" 0.0 :!class /Script/Engine.MaterialInstanceDynamic)
      (Actor|DestroyActor)
      (else
        (Rendering|Material|SetScalarParameterValue (Variables|Default|GetPostProcessMaterial) "Opacity" _output_get :!class /Script/Engine.MaterialInstanceDynamic)))))

(fn ConstructionScript)

(fn Activate
  (params (Speed :type Float%20%28single-precision%29))
  (Variables|Default|Set_FadeInSpeed Speed)
  (Variables|Default|SetIsActive true)
  (return))