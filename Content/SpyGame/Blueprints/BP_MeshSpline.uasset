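; BP_MeshSpline is a construction-time tool that repeats an input mesh along a spline, with no active runtime logic.
; The construction script divides the spline length by SectionLength, dropping any remainder, and adds a spline mesh component per whole section.
; Each component uses the mesh's Z axis as forward, disables decals, applies Scale and takes local-space endpoints and tangents from the spline.
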(event EventBeginPlay)

(event Collision|EventActorBeginOverlap
  (params (OtherActor :type Actor%20Object%20Reference)))

(event EventTick
  (params (DeltaSeconds :type Float%20%28single-precision%29)))

(fn ConstructionScript
  (bind _spline (Variables|Default|GetSpline))
  (bind _spline_2 (Variables|Default|GetSpline))
  (bind _sectionlength (Variables|Default|GetSectionLength))
  (for _index (range 0 (- (Math|Float|Truncate (/ (Spline|GetSplineLength (Variables|Default|GetSpline)) (Variables|Default|GetSectionLength))) 1))
    (bind _returnvalue (AddComponent|AddSplineMeshComponent false))
    (Components|StaticMesh|SetStaticMesh _returnvalue (Variables|Default|GetInputMesh))
    (Rendering|SetReceivesDecals _returnvalue false)
    (SplineMesh|SetForwardAxis _returnvalue "Z" true)
    (Transformation|SetWorldScale3D _returnvalue (Math|Conversions|ToVector(Float) (Variables|Default|GetScale)))
    (SplineMesh|SetStartandEnd _returnvalue (Spline|GetLocationatDistanceAlongSpline _spline_2 (* _index _sectionlength) "Local") (Spline|GetTangentatDistanceAlongSpline _spline_2 (* _index _sectionlength) "Local") (Spline|GetLocationatDistanceAlongSpline _spline (* (+ _index 1) _sectionlength) "Local") (Spline|GetTangentatDistanceAlongSpline _spline (* (+ _index 1) _sectionlength) "Local") true :!class /Script/Engine.SplineMeshComponent)))