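; BP_ElectroGate is an electrified gate that triggers game over when the spy player character overlaps it.
; Open and Close switch the kill radius collision, electricity VFX, emissive glow and ambient audio together, and Toggle flips between them based on the stored state.
; At BeginPlay it creates one dynamic material shared by the top and bottom meshes and marks itself closed.
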(event EventBeginPlay
  (bind _returnvalue (Rendering|Material|CreateDynamicMaterialInstance (Variables|Default|GetElectro_Gate_Bottom) 1 0 "None" :!class /Script/Engine.PrimitiveComponent))
  (bind _output_get (Variables|Default|SetEmissiveMaterial _returnvalue))
  (Rendering|Material|SetMaterial (Variables|Default|GetElectro_Gate_Top) 1 _output_get)
  (Variables|Default|Set_State "NewEnumerator0"))

(event Collision|EventActorBeginOverlap
  (params (OtherActor :type Actor%20Object%20Reference))
  (bind _asbp_spy_game_character (Utilities|Casting|CastToBP_SpyGame_Character OtherActor))
  (Default|GameOver _asbp_spy_game_character "NewEnumerator2"))

(event EventTick
  (params (DeltaSeconds :type Float%20%28single-precision%29)))

(event EventClose
  (Collision|SetCollisionEnabled (Variables|Default|GetKillRadius) "QueryAndPhysics")
  (Rendering|SetVisibility (Variables|Default|GetElectricity_VFX) true true)
  (Rendering|Material|SetVectorParameterValue (Variables|Default|GetEmissiveMaterial) "Color" "(R=0.000000,G=0.391573,B=1.000000,A=1.000000)" :!class /Script/Engine.MaterialInstanceDynamic)
  (Class|AudioComponent|SetPaused (Variables|Default|GetElectro_Gate_Amb) false)
  (Variables|Default|Set_State "NewEnumerator0"))

(event EventOpen
  (Collision|SetCollisionEnabled (Variables|Default|GetKillRadius) "NoCollision")
  (Rendering|SetVisibility (Variables|Default|GetElectricity_VFX) false true)
  (Rendering|Material|SetVectorParameterValue (Variables|Default|GetEmissiveMaterial) "Color" "(R=0.000000,G=0.000000,B=0.000000,A=1.000000)" :!class /Script/Engine.MaterialInstanceDynamic)
  (Class|AudioComponent|SetPaused (Variables|Default|GetElectro_Gate_Amb) true)
  (Variables|Default|Set_State "NewEnumerator2"))

(event EventToggle
  (switch Utilities|FlowControl|Switch|SwitchonE_DoorState (Variables|Default|Get_State)
    (:NewEnumerator0
      (CallFunction|Open))
    (:NewEnumerator2
      (CallFunction|Close))))

(fn ConstructionScript)