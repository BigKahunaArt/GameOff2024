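; BP_DoorPanel is an interactable keypad panel that activates a linked object, presumably a door, when unlocked.
; BeginPlay creates a dynamic screen material, which ActivatewithNotify tints green on success or red when locked.
; Success plays keypad and beep sound bursts around a delay, activates ActivateObject once and disables the box collider.
; Both outcomes report completion to the Notifier, but a locked panel stays interactable.
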(event EventBeginPlay
  (bind _door_panel_01 (Variables|Default|Getdoor-panel-01))
  (bind _returnvalue (Rendering|Material|GetMaterialIndex _door_panel_01 "M_Screen"))
  ;[0 0.2545 1] Startup Logic
  (bind _returnvalue_2 (Rendering|Material|CreateDynamicMaterialInstance (Variables|Default|Getdoor-panel-01) _returnvalue (Utilities|Array|Get(acopy) (Rendering|Material|GetMaterials _door_panel_01) _returnvalue) "None" :!class /Script/Engine.PrimitiveComponent))
  (Variables|Default|SetScreenMaterial _returnvalue_2))

(event EventActivatewithNotify
  (params (Notifier :type I%20Notifier%20Interface))
  ;[1 0.4835 0] Activation logic
  (if (Variables|Default|GetIsUnlocked)
    (if (not (Variables|Default|GetHasActivated))
      (CallFunction|PlaySoundBurstatLocation self "/Game/SpyGame/SFX/4_digit_code.4_digit_code" (Transformation|GetActorLocation) 25.0)
      (Utilities|FlowControl|Delay 2.1)
      (Rendering|Material|SetVectorParameterValue (Variables|Default|GetScreenMaterial) "Color" "(R=0.142538,G=1.000000,B=0.000000,A=1.000000)" :!class /Script/Engine.MaterialInstanceDynamic)
      (Variables|Default|SetHasActivated true)
      (CallFunction|PlaySoundBurstatLocation self "/Game/SpyGame/SFX/beep_accepted.beep_accepted" (Transformation|GetActorLocation) 1e+01)
      (Default|InteractionComplete Notifier)
      (Default|Activate (Variables|Default|GetActivateObject))
      (Collision|SetCollisionEnabled (Variables|Default|GetBox%20Collider) "NoCollision"))
    (else
      (Rendering|Material|SetVectorParameterValue (Variables|Default|GetScreenMaterial) "Color" "(R=1.000000,G=0.004121,B=0.000000,A=1.000000)" :!class /Script/Engine.MaterialInstanceDynamic)
      (CallFunction|PlaySoundBurstatLocation self "/Game/SpyGame/SFX/beep_accepted.beep_accepted" (Transformation|GetActorLocation) 1e+01)
      (Utilities|FlowControl|Delay 0.2)
      (Default|InteractionComplete Notifier))))

(fn ConstructionScript)