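; BP_SecurityGate is a security gate actor that opens and closes instantly by toggling the Gate component's visibility and collision, with a shared sound.
; A DoorState check guards OpenDoor and CloseDoor against repeat calls, and IsClosed selects the state requested at BeginPlay.
; Open, Close and Toggle act after short delays.
; Activate also delays, then requests the opposite of IsClosed rather than reading DoorState.
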(event Custom|CloseDoor
  (bind _gate (Variables|Default|GetGate))
  (if (Utilities|Enum|Equal(Enum) (Variables|Default|Get_DoorState) "NewEnumerator2")
    (Rendering|SetVisibility _gate true true)
    (Collision|SetCollisionEnabled _gate "QueryAndPhysics")
    (Variables|Default|Set_DoorState "NewEnumerator0")
    (Audio|PlaySoundatLocation "/Game/SpyGame/SFX/SecurityDoor_OpenClose.SecurityDoor_OpenClose" (Transformation|GetActorLocation) "0, 0, 0" 1.0 1.0 0.0 0 0 0)))

(event Custom|OpenDoor
  (bind _gate (Variables|Default|GetGate))
  (if (Utilities|Enum|Equal(Enum) (Variables|Default|Get_DoorState) "NewEnumerator0")
    (Rendering|SetVisibility _gate false true)
    (Collision|SetCollisionEnabled _gate "NoCollision")
    (Variables|Default|Set_DoorState "NewEnumerator2")
    (Audio|PlaySoundatLocation "/Game/SpyGame/SFX/SecurityDoor_OpenClose.SecurityDoor_OpenClose" (Transformation|GetActorLocation) "0, 0, 0" 1.0 1.0 0.0 0 0 0)))

(event EventBeginPlay
  (if (Variables|Default|GetIsClosed)
    (CallFunction|CloseDoor)
    (else
      (CallFunction|OpenDoor))))

(event Collision|EventActorBeginOverlap
  (params (OtherActor :type Actor%20Object%20Reference)))

(event EventTick
  (params (DeltaSeconds :type Float%20%28single-precision%29)))

(event EventActivate
  (Utilities|FlowControl|Delay 0.5)
  (if (Variables|Default|GetIsClosed)
    (CallFunction|OpenDoor)
    (else
      (CallFunction|CloseDoor))))

(event EventClose
  (Utilities|FlowControl|Delay 0.2)
  (CallFunction|CloseDoor))

(event EventOpen
  (Utilities|FlowControl|Delay 0.2)
  (CallFunction|OpenDoor))

(event EventToggle
  (Utilities|FlowControl|Delay 0.2)
  (switch Utilities|FlowControl|Switch|SwitchonE_DoorState (Variables|Default|Get_DoorState)
    (:NewEnumerator0
      (CallFunction|OpenDoor))
    (:NewEnumerator2
      (CallFunction|CloseDoor))))

(fn ConstructionScript)