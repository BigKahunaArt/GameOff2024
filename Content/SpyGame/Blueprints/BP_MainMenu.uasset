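; BP_MainMenu is a main menu actor that periodically triggers a glitch effect and toggles a set of decals.
; BeginPlay hides every entry in the Decal array and starts a looping timer with a randomized initial delay.
; Each tick of that timer spawns BP_GlitchScreenEffect at the actor's transform, then a FlipFlop alternately shows and hides the decals through their root components.
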(event Custom|CustomEvent_0
  (Game|SpawnActorfromClass "/Game/SpyGame/Blueprints/BP_GlitchScreenEffect.BP_GlitchScreenEffect_C" (Transformation|GetActorTransform) "Undefined" 0 0)
  (Utilities|FlowControl|FlipFlop
    (:A
      (for _array_element (Variables|Default|GetDecal)
        (Rendering|SetVisibility (Variables|/Script/Engine.Actor|GetRootComponent _array_element) true true)))
    (:B
      (for _array_element_2 (Variables|Default|GetDecal)
        (Rendering|SetVisibility (Variables|/Script/Engine.Actor|GetRootComponent _array_element_2) false true)))))

(event EventBeginPlay
  (for _array_element (Variables|Default|GetDecal)
    (Rendering|SetVisibility (Variables|/Script/Engine.Actor|GetRootComponent _array_element) false false))
  (Utilities|Time|SetTimerbyEvent (delegate Custom|CustomEvent_0) 8.0 true 5.0 5.0))

(event Collision|EventActorBeginOverlap
  (params (OtherActor :type Actor%20Object%20Reference)))

(event EventTick
  (params (DeltaSeconds :type Float%20%28single-precision%29)))

(fn ConstructionScript)