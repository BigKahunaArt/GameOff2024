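; BF_SpyGame is a Blueprint function library of shared cosmetic helpers for SpyGame.
; PlaySoundBurstAtLocation plays a sound with slightly randomized volume and pitch, then spawns a one-shot Niagara ring burst there, sized through its RingSize variable.
; Two random-roll helpers return true about one third or two thirds of the time, named as intended for non-gameplay use.
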(fn PlaySoundBurstatLocation
  (params (Owner :type Actor%20Object%20Reference) (Sound :type Sound%20Base%20Object%20Reference) (Location :type Vector) (BurstSize :type Float%20%28single-precision%29))
  (Audio|PlaySoundatLocation Owner Sound Location "0, 0, 0" (Math|Random|RandomFloatinRange 1.0 1.2) (Math|Random|RandomFloatinRange 0.85 1.0) 0.0 0 0 0)
  (bind _returnvalue (Niagara|SpawnSystematLocation Owner "/Game/SpyGame/VFX/NS_RingBurstOnce.NS_RingBurstOnce" Location))
  (Niagara|SetNiagaraVariable(Float) _returnvalue "RingSize" BurstSize))

(fn NonGameplayLowProbability
  (return (< (Math|Random|RandomFloatinRange 0.0 1.0) 0.33)))

(fn NonGameplayHighProbability
  (return (< (Math|Random|RandomFloatinRange 0.0 1.0) 0.66)))