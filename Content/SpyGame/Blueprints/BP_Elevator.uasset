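; BP_Elevator is an elevator actor that serves as a transition to another level.
; On BeginPlay it disables its interaction collider if no valid NextLevel is set.
; Both activation events share one path that, given a valid NextLevel, spawns and activates a BP_FadeOut, waits briefly, then opens that level by object reference.
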(event EventBeginPlay
  (Variables|Default|GetNextLevel
    (:then)
    (:else
      (Collision|SetCollisionEnabled (Variables|Default|GetInteractionCollider) "NoCollision"))))

(event Collision|EventActorBeginOverlap
  (params (OtherActor :type Actor%20Object%20Reference)))

(event EventTick
  (params (DeltaSeconds :type Float%20%28single-precision%29)))

(event EventActivate
  (bind _nextlevel (Variables|Default|GetNextLevel)
    (:then
      (bind _returnvalue (Game|SpawnActorfromClass "/Game/SpyGame/Blueprints/BP_FadeOut.BP_FadeOut_C" (Transformation|GetActorTransform) "Undefined" 0 0))
      (Default|Activate _returnvalue 75.0)
      (Utilities|FlowControl|Delay 3.0)
      (Game|OpenLevel(byObjectReference) _nextlevel))
    (:else)))

(event EventActivatewithNotify
  (params (Notifier :type I%20Notifier%20Interface))
  (bind _nextlevel (Variables|Default|GetNextLevel)
    (:then
      (bind _returnvalue (Game|SpawnActorfromClass "/Game/SpyGame/Blueprints/BP_FadeOut.BP_FadeOut_C" (Transformation|GetActorTransform) "Undefined" 0 0))
      (Default|Activate _returnvalue 75.0)
      (Utilities|FlowControl|Delay 3.0)
      (Game|OpenLevel(byObjectReference) _nextlevel))
    (:else)))

(fn ConstructionScript)