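; Scripted swing action event that triggers when the spy character overlaps it at speed.
; A dummy mesh plays the run-and-swing montage while the hidden player teleports to the start and flies slowly along, with occasional bullet time.
; The montage notify snaps the player to the end point and restores walking, then drops the grab point with crash audio before delayed self-destruction.
; A looping timer randomises the hook's yaw jiggle, interpolated on Tick.
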(event Custom|CustomEvent_0
  (Variables|Default|SetHookJiggleRot (Math|Random|RandomFloatinRange -2e+01 2e+01)))

(event EventBeginPlay
  (Audio|Components|Audio|Stop (Variables|Default|Getlight-metal-crash-6765_Cue))
  ;[1 1 1] Hide the dummy mesh
  (Rendering|SetVisibility (Variables|Default|GetDummyMesh) false true)
  (Utilities|Time|SetTimerbyEvent (delegate Custom|CustomEvent_0) 5.0 true))

(event Collision|EventActorBeginOverlap
  (params (OtherActor :type Actor%20Object%20Reference))
  ;[1 1 1] Get the player blueprint / check for player
  (bind _asbp_spy_game_character (Utilities|Casting|CastToBP_SpyGame_Character OtherActor))
  (if (> (Math|Vector|VectorLength (Variables|/Script/Engine.MovementComponent|GetVelocity (Pawn|GetMovementComponent _asbp_spy_game_character))) 2e+02)
    (Variables|Default|SetPlayerCharacter _asbp_spy_game_character)
    (CallFunction|Activate)
    (Animation|Montage|PlayMontage (Variables|Default|GetDummyMesh) "/Game/SpyGame/Models/Agent/Animations/AGENT_Run_And_Swing_Montage.AGENT_Run_And_Swing_Montage" 0.9 0.1
      (:then
        ;[1 1 1] Hide the player mesh and snap to the origin of the animation
        (Rendering|SetVisibility (Variables|/Script/Engine.Character|GetMesh (Variables|Default|GetPlayerCharacter)) false false)
        (Transformation|SetWorldLocation (Variables|/Script/Engine.Character|GetCapsuleComponent (Variables|Default|GetPlayerCharacter)) (Transformation|GetWorldLocation (Variables|Default|GetStartPoint)) false true)
        (bind _success (CallFunction|NonGameplayLowProbability))
        (if _success
          ;[1 1 1] Bullet time
          (Utilities|FlowControl|Delay 0.75)
          (Utilities|Time|SetGlobalTimeDilation 0.1)
          (Utilities|FlowControl|Delay 0.02)
          (Utilities|FlowControl|Delay 0.02)
          (Utilities|Time|SetGlobalTimeDilation 1.0)))
      (:OnNotifyBegin
        ;[1 1 1] When the animation event fires snap the player to the end point and turn it on again
        (Rendering|SetVisibility (Variables|Default|GetDummyMesh) false true)
        (Transformation|SetWorldLocation (Variables|/Script/Engine.Character|GetCapsuleComponent (Variables|Default|GetPlayerCharacter)) (Transformation|GetWorldLocation (Variables|Default|GetEndPoint)) false true)
        (Rendering|SetVisibility (Variables|/Script/Engine.Character|GetMesh (Variables|Default|GetPlayerCharacter)) true true)
        (Variables|Default|Set_Activated false)
        (Pawn|Components|CharacterMovement|SetMovementMode (Variables|/Script/Engine.Character|GetCharacterMovement (Variables|Default|GetPlayerCharacter)) "MOVE_Walking" 0)
        (Pawn|Input|AddMovementInput (Variables|Default|GetPlayerCharacter) "0.000000,-10.000000, 0" 5.0 false)
        (Variables|Default|Set_DropGrabPoint true)
        (Audio|Components|Audio|Stop (Variables|Default|Getmetal-chain-7056_Cue))
        (Audio|Components|Audio|Play (Variables|Default|Getlight-metal-crash-6765_Cue) 0.0)
        (Utilities|FlowControl|Delay 45.0)
        (Actor|DestroyActor)))))

(event EventTick
  (params (DeltaSeconds :type Float%20%28single-precision%29))
  (bind _grabpoint (Variables|Default|GetGrabPoint))
  (bind _grabpoint_2 (Variables|Default|GetGrabPoint))
  (bind _returnvalue (Transformation|GetWorldLocation _grabpoint))
  (Utilities|FlowControl|Sequence
    (:then_0
      (bind _playercharacter (Variables|Default|GetPlayerCharacter)
        (:then
          ;[1 1 1] While the animation is playing move the player slowly towards the end point (roughly in time with the animation)
          (if (Variables|Default|Get_Activated)
            (Pawn|Components|CharacterMovement|SetMovementMode (Variables|/Script/Engine.Character|GetCharacterMovement _playercharacter) "MOVE_Flying" 0)
            (Variables|/Script/Engine.CharacterMovementComponent|SetMaxFlySpeed (Variables|/Script/Engine.Character|GetCharacterMovement _playercharacter) (Variables|Default|GetCameraPanSpeed))
            (Pawn|Input|AddMovementInput _playercharacter "0.000000,-1.000000, 0" 1.0 false)))
        (:else)))
    (:then_1
      (if (Variables|Default|Get_DropGrabPoint)
        (Transformation|SetWorldLocation _grabpoint (Math|Vector|MakeVector (.x _returnvalue) (.y _returnvalue) (+ (* DeltaSeconds -9.5e+02) (.z _returnvalue))) false false)))
    (:then_2
      (Transformation|SetWorldRotation _grabpoint_2 (Math|Interpolation|RInterpTo (Transformation|GetWorldRotation _grabpoint_2) (Math|Rotator|MakeRotator 0.0 0.0 (Variables|Default|GetHookJiggleRot)) DeltaSeconds 0.2) false false))))

(event Collision|EventActorEndOverlap
  (params (OtherActor :type Actor%20Object%20Reference))
  (Utilities|Casting|CastToBP_SpyGame_Character OtherActor))

(fn ConstructionScript
  (bind _dummymesh (Variables|Default|GetDummyMesh))
  ;[1 1 1] For some stupid reason there is a bug in the animation and this is required to fix it
  (Components|Animation|SetAnimationMode _dummymesh "AnimationSingleNode")
  (Variables|/Script/Engine.SkeletalMeshComponent|SetAnimationData _dummymesh (Utilities|Struct|MakeSingleAnimationPlayData "/Game/SpyGame/Models/Agent/Animations/AGENT_Run_And_Swing.AGENT_Run_And_Swing" false false 0.0)))

(fn Activate
  (Variables|Default|Set_Activated true)
  (Rendering|SetVisibility (Variables|Default|GetDummyMesh) true true)
  ;[1 1 1] Kill the player's velocity
  (Variables|/Script/Engine.MovementComponent|SetVelocity (Pawn|GetMovementComponent (Variables|Default|GetPlayerCharacter)) "0, 0, 0")
  (Development|PrintString "Action event activate")
  (return))