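; BP_TestAI is a Grinner enemy in the spy game that patrols a spline path and ends the game when it spots the player.
; Once activated, Tick advances it along the spline, looping or halting at the end, and jitters it vertically while halted.
; A forward sphere trace detects an unhidden player, halts it, flashes randomly tinted lightning meshes, plays attack sounds and calls GameOver.
; A looping timer with a randomized interval plays laugh barks.
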(event Custom|Bark
  ;[1 1 1] Bark
  (Audio|PlaySoundatLocation "/Game/SpyGame/SFX/Grinner_Laugh_Rand.Grinner_Laugh_Rand" (Transformation|GetActorLocation) "0, 0, 0" 1.0 1.0 0.0 0 0 0))

(event Custom|Jiggle
  (params (DeltaTime :type Float%20%28single-precision%29))
  (bind _enemy_grinner_01 (Variables|Default|Getenemy_grinner_01))
  (bind _returnvalue (Transformation|GetWorldLocation _enemy_grinner_01))
  ;[1 1 1] Jiggle
  (Variables|Default|Set_Halt true)
  (Transformation|SetWorldLocation _enemy_grinner_01 (Math|Vector|MakeVector (.x _returnvalue) (.y _returnvalue) (+ (.z (.location (Spline|GetTransformatDistanceAlongSpline (Variables|/Game/SpyGame/Blueprints/BP_AIPath.BP_AIPath_C|GetSpline (Variables|Default|GetPath)) (Variables|Default|Get_SplineDistance) "World" false))) (* (Math|Random|RandomFloatinRange -7.5 7.5) (* DeltaTime 5e+01)))) false false))

(event EventBeginPlay
  (bind _returnvalue (Math|Random|RandomFloatinRange 0.0 1.0))
  (bind _returnvalue_2 (Math|Color|Lerp(LinearColor) "(R=1.000000,G=0.239747,B=0.000000,A=1.000000)" "(R=1.000000,G=0.000000,B=0.000000,A=1.000000)" _returnvalue))
  (Utilities|Time|SetTimerbyEvent (delegate Custom|Bark) (Math|Random|RandomFloatinRange 1e+01 2e+01) true)
  (Variables|Default|SetVFXEffectMesh (Utilities|Array|MakeArray (Variables|Default|GetLightningEffect) (Variables|Default|GetLightningEffectSide)))
  ;[1 1 1] SetRandomColor
  (bind _returnvalue_3 (Rendering|Material|CreateDynamicMaterialInstance (Variables|Default|GetLightningEffect) 0 "/Game/SpyGame/Materials/M_Electricity_Grinner_Inst.M_Electricity_Grinner_Inst" "None" :!class /Script/Engine.PrimitiveComponent))
  (Rendering|Material|SetVectorParameterValue _returnvalue_3 "Color" _returnvalue_2 :!class /Script/Engine.MaterialInstanceDynamic)
  (bind _returnvalue_4 (Rendering|Material|CreateDynamicMaterialInstance (Variables|Default|GetLightningEffectSide) 0 "/Game/SpyGame/Materials/M_Electricity_Grinner_Inst.M_Electricity_Grinner_Inst" "None" :!class /Script/Engine.PrimitiveComponent))
  (Rendering|Material|SetVectorParameterValue _returnvalue_4 "Color" _returnvalue_2 :!class /Script/Engine.MaterialInstanceDynamic)
  (for _array_element (Variables|Default|GetVFXEffectMesh)
    (Rendering|SetVisibility _array_element false false)))

(event EventActivate
  (Variables|Default|Set_Active true))

(event EventTick
  (params (DeltaSeconds :type Float%20%28single-precision%29))
  (bind _enemy_grinner_01 (Variables|Default|Getenemy_grinner_01))
  (bind _vfxeffectmesh (Variables|Default|GetVFXEffectMesh))
  (bind _returnvalue (Transformation|GetWorldLocation _enemy_grinner_01))
  (if (Variables|Default|Get_Active)
    (Utilities|FlowControl|Sequence
      (:then_0
        (if (Variables|Default|Get_Halt)
          (CallFunction|Jiggle DeltaSeconds)
          (else
            ;[1 1 1] Handle Spline
            (bind _output_get (Variables|Default|Set_SplineDistance (+ (* DeltaSeconds (Variables|Default|GetSpeed)) (Variables|Default|Get_SplineDistance))))
            (Transformation|SetWorldLocationAndRotation (Variables|Default|Getenemy_grinner_01) (.location (Spline|GetTransformatDistanceAlongSpline (Variables|/Game/SpyGame/Blueprints/BP_AIPath.BP_AIPath_C|GetSpline (Variables|Default|GetPath)) _output_get "World" false)) (.rotation (Spline|GetTransformatDistanceAlongSpline (Variables|/Game/SpyGame/Blueprints/BP_AIPath.BP_AIPath_C|GetSpline (Variables|Default|GetPath)) _output_get "World" false)) false false)
            (if (>= _output_get (Spline|GetSplineLength (Variables|/Game/SpyGame/Blueprints/BP_AIPath.BP_AIPath_C|GetSpline (Variables|Default|GetPath))))
              (if (Variables|Default|Get_NoLoopPath)
                (Variables|Default|Set_Halt true)
                (else
                  (Variables|Default|Set_SplineDistance 0.0)))))))
      (:then_1
        (if (not (Variables|Default|Get_Halt))
          (bind (_outhit _returnvalue_2) (Collision|SphereTraceByChannel _returnvalue (+ _returnvalue (* (Math|Vector|GetForwardVector _enemy_grinner_01) (Variables|Default|GetTraceDistance))) (Variables|Default|GetTraceRadius) "TraceTypeQuery3" true 0 "None"))
          (if _returnvalue_2
            (bind _asbp_spy_game_character (Utilities|Casting|CastToBP_SpyGame_Character (.HitActor (Collision|BreakHitResult _outhit))))
            (bind _hidden (Default|PlayerIsHidden _asbp_spy_game_character))
            (if (not _hidden)
              (Variables|Default|Set_Halt true)
              (for _array_element _vfxeffectmesh
                (Rendering|SetVisibility _array_element true false)
                (Audio|PlaySoundatLocation "/Game/SpyGame/SFX/Grinner_Laugh_Rand.Grinner_Laugh_Rand" (.Location (Collision|BreakHitResult _outhit)) "0, 0, 0" 1.0 1.0 0.0 0 0 0)
                (Audio|PlaySoundatLocation "/Game/SpyGame/SFX/Grinner_Electro_Attack.Grinner_Electro_Attack" (.Location (Collision|BreakHitResult _outhit)) "0, 0, 0" 1.0 1.0 0.0 0 0 0)
                (Default|GameOver _asbp_spy_game_character "NewEnumerator2")
                (Utilities|FlowControl|Delay (Math|Random|RandomFloatinRange 0.2 0.35))
                (for _array_element_2 _vfxeffectmesh
                  (Rendering|SetVisibility _array_element_2 false false))))))))))

(fn ConstructionScript)