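; BP_Trigger_Music is a placeable trigger volume that plays an assigned music track when the spy game player character overlaps it.
; After a short random delay it plays the track as 2D sound through a shared music concurrency setting.
; An optional trigger-once flag disables the box collision after the first play.
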(event EventBeginPlay
  (Variables|Default|Set_HasTriggered false))

(event Collision|EventActorBeginOverlap
  (params (OtherActor :type Actor%20Object%20Reference))
  (Utilities|Casting|CastToBP_SpyGame_Character OtherActor)
  (bind _music (Variables|Default|GetMusic)
    (:then
      ;[1 1 1] Don't trigger it immediately
      (Utilities|FlowControl|Delay (Math|Random|RandomFloatinRange 0.1 0.3))
      (Audio|PlaySound2D _music 1.0 1.0 0.0 "/Game/SpyGame/SFX/MusicSoundConcurrency.MusicSoundConcurrency" 0)
      (Variables|Default|Set_HasTriggered true)
      (if (Variables|Default|GetTriggerOnce)
        (Collision|SetCollisionEnabled (Variables|Default|GetBox) "NoCollision")))
    (:else)))

(event EventTick
  (params (DeltaSeconds :type Float%20%28single-precision%29)))

(fn ConstructionScript)