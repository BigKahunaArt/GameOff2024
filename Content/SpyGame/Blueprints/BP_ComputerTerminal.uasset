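; BP_ComputerTerminal is an interactable retro computer terminal that shows the player an email.
; BeginPlay creates a dynamic CRT screen material, which activation recolors to amber text on black.
; ActivatewithNotify opens W_ComputerTerminal with the email text and starts a looping timer that polls until the widget leaves the viewport.
; On close, it clears the timer, tells the notifier the interaction is complete and optionally enables a linked object.
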(event Custom|CheckUI_Closed
  ;[1 1 1] Wait for the player to close the widget
  (if (not (UserInterface|Viewport|IsinViewport (Variables|Default|Get_EmailWidget)))
    (Utilities|Time|ClearandInvalidateTimerbyHandle (Variables|Default|Get_CheckUIDone_Handle))
    (Default|InteractionComplete (Variables|Default|Get_INotifyPlayer))
    (if (Variables|Default|GetCanEnableObject)
      (Default|Enable (Variables|Default|GetEnableObjectOnRead)))))

(event EventBeginPlay
  (bind _returnvalue (Rendering|Material|CreateDynamicMaterialInstance (Variables|Default|Getretro_screen_prop) 1 "/Game/SpyGame/Models/Props/Screen/M_CrtScreen.M_CrtScreen" "None" :!class /Script/Engine.PrimitiveComponent))
  (Variables|Default|SetCRTScreen _returnvalue))

(event Collision|EventActorBeginOverlap
  (params (OtherActor :type Actor%20Object%20Reference)))

(event EventTick
  (params (DeltaSeconds :type Float%20%28single-precision%29)))

(event EventActivatewithNotify
  (params (Notifier :type I%20Notifier%20Interface))
  (bind _crtscreen (Variables|Default|GetCRTScreen))
  ;[1 1 1] Create the email widget
  (Variables|Default|Set_INotifyPlayer Notifier)
  (bind _returnvalue (UserInterface|CreateWidget "/Game/SpyGame/UI/Widgets/W_ComputerTerminal.W_ComputerTerminal_C" (Game|GetPlayerController 0)))
  (bind _output_get (Variables|Default|Set_EmailWidget _returnvalue))
  (Default|SetEmailText _output_get (Variables|Default|GetEmailText))
  (UserInterface|Viewport|AddtoViewport _output_get 0)
  (bind _returnvalue_2 (Utilities|Time|SetTimerbyEvent (delegate Custom|CheckUI_Closed) 1.0 true 0.2))
  (Variables|Default|Set_CheckUIDone_Handle _returnvalue_2)
  (Rendering|Material|SetVectorParameterValue _crtscreen "BackgroundColor" "(R=0.000000,G=0.000000,B=0.000000,A=1.000000)" :!class /Script/Engine.MaterialInstanceDynamic)
  (Rendering|Material|SetVectorParameterValue _crtscreen "TextColor" "(R=1.000000,G=0.746285,B=0.000000,A=1.000000)" :!class /Script/Engine.MaterialInstanceDynamic))

(fn ConstructionScript)