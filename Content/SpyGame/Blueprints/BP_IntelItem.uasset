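; BP_IntelItem is an intel pickup that shows its text as an email in a computer terminal widget when activated.
; ActivatewithNotify stores the notifier, plays a sound and, after a short delay, fills W_ComputerTerminal with IntelText and adds it to the viewport.
; A looping timer polls until the widget leaves the viewport, then calls InteractionComplete on the notifier and destroys the actor.
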(event Custom|CheckUI_Closed
  ;[1 1 1] Wait for the player to close the widget
  (if (not (UserInterface|Viewport|IsinViewport (Variables|Default|Get_EmailWidget)))
    (Utilities|Time|ClearandInvalidateTimerbyHandle (Variables|Default|Get_CheckUIDone_Handle))
    (Default|InteractionComplete (Variables|Default|Get_INotifyPlayer))
    (Actor|DestroyActor)))

(event EventBeginPlay)

(event Collision|EventActorBeginOverlap
  (params (OtherActor :type Actor%20Object%20Reference)))

(event EventTick
  (params (DeltaSeconds :type Float%20%28single-precision%29)))

(event EventActivatewithNotify
  (params (Notifier :type I%20Notifier%20Interface))
  ;[1 1 1] Create the email widget
  (Variables|Default|Set_INotifyPlayer Notifier)
  (bind _returnvalue (UserInterface|CreateWidget "/Game/SpyGame/UI/Widgets/W_ComputerTerminal.W_ComputerTerminal_C" (Game|GetPlayerController 0)))
  (bind _output_get (Variables|Default|Set_EmailWidget _returnvalue))
  (Audio|PlaySound2D "/Game/SpyGame/SFX/energy-up-sound-effect-230472.energy-up-sound-effect-230472" 1.0 1.0 0.0 0 0)
  (Utilities|FlowControl|Delay 0.75)
  (Default|SetEmailText _output_get (Variables|Default|GetIntelText))
  (UserInterface|Viewport|AddtoViewport _output_get 0)
  (bind _returnvalue_2 (Utilities|Time|SetTimerbyEvent (delegate Custom|CheckUI_Closed) 1.0 true 0.2))
  (Variables|Default|Set_CheckUIDone_Handle _returnvalue_2))

(fn ConstructionScript)