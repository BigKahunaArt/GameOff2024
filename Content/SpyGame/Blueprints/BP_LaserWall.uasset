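; BP_LaserWall is a moving security laser that activates a Device when the player character moves while overlapping it.
; Tick sweeps the wall back and forth along world Y, flipping Impulse whenever the travelled Distance exceeds Offset.
; Overlap events store or clear the player reference and play or fade out the beam hover sound.
; Tick also checks that player's velocity, so standing still inside the beam does not activate the Device.
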(event EventBeginPlay
  (Variables|Default|Set_StartingPosition (Transformation|GetActorLocation))
  (Audio|Components|Audio|Stop (Variables|Default|GetSecurityBeam_Hover)))

(event Collision|EventActorBeginOverlap
  (params (OtherActor :type Actor%20Object%20Reference))
  (bind _asbp_spy_game_character (Utilities|Casting|CastToBP_SpyGame_Character OtherActor))
  (Variables|Default|SetPlayerCharacter _asbp_spy_game_character)
  (Audio|Components|Audio|Play (Variables|Default|GetSecurityBeam_Hover) 0.0))

(event EventTick
  (params (DeltaSeconds :type Float%20%28single-precision%29))
  (bind _returnvalue (Transformation|GetActorLocation))
  (Utilities|FlowControl|Sequence
    (:then_0
      ;[1 1 1] Movement Code
      (if (> (Variables|Default|Get_Distance) (Variables|Default|GetOffset))
        (Variables|Default|SetImpulse (* (Variables|Default|GetImpulse) -1.0))
        (Variables|Default|Set_Distance 0.0)
        (else
          (Variables|Default|Set_Distance (+ (Variables|Default|Get_Distance) (* DeltaSeconds (Variables|Default|GetSpeed))))
          (Transformation|SetActorLocation (Math|Vector|MakeVector (.x _returnvalue) (+ (.y _returnvalue) (* DeltaSeconds (* (Variables|Default|GetSpeed) (Variables|Default|GetImpulse)))) (.z _returnvalue)) false false))))
    (:then_1
      (Variables|Default|GetPlayerCharacter
        (:then
          (if (> (Math|Vector|VectorLength (Transformation|GetVelocity (Variables|Default|GetPlayerCharacter))) 1.0)
            (Default|Activate (Variables|Default|GetDevice))))
        (:else)))))

(event Collision|EventActorEndOverlap
  (params (OtherActor :type Actor%20Object%20Reference))
  (Utilities|Casting|CastToBP_SpyGame_Character OtherActor)
  (Variables|Default|SetPlayerCharacter 0)
  (Audio|Components|Audio|FadeOut (Variables|Default|GetSecurityBeam_Hover) 0.1 0.0 "Linear" :!class /Script/Engine.AudioComponent))

(fn ConstructionScript)