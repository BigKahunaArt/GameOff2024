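; BP_FadeOut is a screen fade-out actor that drives a post-process material's Opacity and can restart the current level afterward.
; BeginPlay creates a dynamic instance of PP_FadeOut and adds it as a blendable.
; Activate or FadeOutRestartLevel sets the speed and starts Tick interpolating Alpha, with interp speed also scaled by delta time.
; At 0.9, Tick snaps opacity to full, deactivates, and reopens the level if flagged.
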(event EventBeginPlay
  (Variables|Default|Set_Alpha 0.0)
  (Variables|Default|SetIsActive false)
  (bind _returnvalue (Rendering|Material|CreateDynamicMaterialInstance "/Game/SpyGame/Engine/PostProcessing/PP_FadeOut.PP_FadeOut" "None" "None" :!class /Script/Engine.KismetMaterialLibrary))
  (bind _output_get (Variables|Default|SetPostProcessMaterial _returnvalue))
  (Rendering|Material|SetScalarParameterValue _output_get "Opacity" 0.0 :!class /Script/Engine.MaterialInstanceDynamic)
  (Rendering|AddorUpdateBlendable (Variables|Default|GetPostProcess) _output_get 1.0 :!class /Script/Engine.PostProcessComponent))

(event EventTick
  (params (DeltaSeconds :type Float%20%28single-precision%29))
  (if (< (Variables|Default|Get_Alpha) 0.9)
    (if (Variables|Default|GetIsActive)
      (bind _output_get (Variables|Default|Set_Alpha (Math|Interpolation|FInterpTo (Variables|Default|Get_Alpha) 1.0 DeltaSeconds (* DeltaSeconds (Variables|Default|Get_FadeOutSpeed)))))
      (Rendering|Material|SetScalarParameterValue (Variables|Default|GetPostProcessMaterial) "Opacity" _output_get :!class /Script/Engine.MaterialInstanceDynamic))
    (else
      (Rendering|Material|SetScalarParameterValue (Variables|Default|GetPostProcessMaterial) "Opacity" 1.0 :!class /Script/Engine.MaterialInstanceDynamic)
      (Variables|Default|SetIsActive false)
      (if (Variables|Default|Get_RestartLevel)
        (bind _returnvalue (Game|GetCurrentLevelName true))
        (Game|OpenLevel(byName) (Utilities|String|StringToName _returnvalue))))))

(fn ConstructionScript)

(fn Activate
  (params (Speed :type Float%20%28single-precision%29))
  (Variables|Default|Set_FadeOutSpeed Speed)
  (Variables|Default|SetIsActive true)
  (return))

(fn FadeOutRestartLevel
  (params (Speed :type Float%20%28single-precision%29))
  (Variables|Default|Set_FadeOutSpeed Speed)
  (Variables|Default|SetIsActive true)
  (Variables|Default|Set_RestartLevel true)
  (return))